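; BP_MakeTile is a grid generator actor that spawns a field of BP_Tile actors around its own location.
; MakeTile destroys previously tracked tiles through ClearTiles, then runs nested X and Y loops, spacing new tiles by Size and storing them in Tiles.
; GetMakeStartPos offsets the origin by half the grid extent.
; Tiles copy the actor's rotation, but their positions stay on world axes, and no event here calls MakeTile.
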(fn `ClearTiles`
  (if (`KismetArrayLibrary.Array_IsNotEmpty` (`self.Tiles`))
    (for _array_element (`self.Tiles`)
      (`self.K2_DestroyActor` _array_element))
    (`KismetArrayLibrary.Array_Clear` (`self.Tiles`))))

(fn `GetMakeStartPos`
  (returns (StartPose :type "Vector Structure"))
  (bind (_returnvalue_x _returnvalue_y _returnvalue_z) (`KismetMathLibrary.BreakVector` (`self.K2_GetActorLocation`)))
  (return (`KismetMathLibrary.MakeVector` (- _returnvalue_x (/ (* (`self.X`) (`self.Size`)) 2.0)) (- _returnvalue_y (/ (* (`self.Y`) (`self.Size`)) 2.0)) _returnvalue_z)))

(fn `MakeTile`
  (`self.ClearTiles`)
  (for _index (range (+ (`self.X`) 1))
    (for _index_2 (range (+ (`self.Y`) 1))
      ; Comment
      (bind _returnvalue (`|SpawnActorFromClass` "/Game/TileContents/BP_Tile.BP_Tile_C" (`KismetMathLibrary.MakeTransform` (+ (`KismetMathLibrary.MakeVector` (* _index (`self.Size`)) (* _index_2 (`self.Size`))) (`self.GetMakeStartPos`)) (`self.K2_GetActorRotation`)) "Undefined" "MultiplyWithRoot" null null))
      (`KismetArrayLibrary.Array_Add` (`self.Tiles`) _returnvalue))))

(fn `UserConstructionScript`)