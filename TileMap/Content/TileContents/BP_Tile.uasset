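; BP_Tile is a tile actor that disappears one second after a third-person character touches its trigger box.
; The box starts without collision and binds to the BP_GS game state update dispatcher, with ChangeGS enabling query and physics collision when the passed state matches.
; Overlap handling runs only on the server, which destroys the actor after the delay.
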(event `self.ReceiveBeginPlay`
  (`PrimitiveComponent.SetCollisionEnabled` (`self.Box`) "NoCollision")
  (bind _asbp_gs (cast `/Game/GMB/Game/BP_GS` (`GameplayStatics.GetGameState`)))
  (add `/Game/GMB/Game/BP_GS.DS_UpdateGS` _asbp_gs (`|CreateDelegate` :!event `ChangeGS`)))

(event `self.Box.OnComponentBeginOverlap`
  (params (OverlappedComponent :type "PrimitiveComponent Object Reference") (OtherActor :type "Actor Object Reference") (OtherComp :type "PrimitiveComponent Object Reference") (OtherBodyIndex :type Integer) (bFromSweep :type Boolean) (SweepResult :type "HitResult Structure (by ref)"))
  (`/Engine/EditorBlueprintResources/ActorMacros.Switch Has Authority`
    (:`Authority`
      (cast `/Game/GMB/Game/BP_ThirdPersonCharacter` OtherActor)
      (`KismetSystemLibrary.Delay` 1.0)
      (`self.K2_DestroyActor`))))

(fn `ChangeGS`
  (params (NewParam :type "/Game/GMB/EN_GS Enum" :default "NewEnumerator0"))
  (if (`|EnumEquality` NewParam (`self.GS`))
    (`PrimitiveComponent.SetCollisionEnabled` (`self.Box`) "QueryAndPhysics")))

(fn `UserConstructionScript`)