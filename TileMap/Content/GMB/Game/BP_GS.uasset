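; BP_GS holds the replicated game phase (GS) and a per-phase time value, broadcasting both through event dispatchers.
; ChangeGS sets the phase and zeroes Deltasec, while OnRep_GS broadcasts phase changes.
; Tick routes Ready and Play to identical handlers that update Deltasec on authority, then broadcast it on every machine, covering listen-server hosts.
; That update multiplies by delta time rather than adding, so Deltasec stays zero after a reset.
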(event `self.ReceiveTick`
  (params (DeltaSeconds :type "Float (single-precision)"))
  (switch `/Game/GMB/EN_GS` (`self.GS`)
    (:`NewEnumerator1`
      (`self.TickReady` DeltaSeconds))
    (:`NewEnumerator2`
      (`self.TickPlay` DeltaSeconds))))

(fn `ChangeGS`
  (params (GS :type "/Game/GMB/EN_GS Enum" :default "NewEnumerator0"))
  (set `self.GS` GS)
  ; 상태 변경시마다 초 초기화
  (set `self.Deltasec` 0.0))

(fn `OnRep_GS`
  (`self.DS_UpdateGS` (`self.GS`)))

(fn `TickPlay`
  (params (DeltaSec :type "Float (single-precision)"))
  (`|ExecutionSequence`
    (:`then_0`
      (`/Engine/EditorBlueprintResources/ActorMacros.Switch Has Authority`
        (:`Authority`
          (set `self.Deltasec` (* DeltaSec (`self.Deltasec`))))))
    (:`then_1`
      ; 리슨서버- 다 보내야하는 정보:
      ; 서버 자체도 클라여서 ㅇ시퀀ㄱ스연결
      (`self.DS_DeltaSec` (`self.Deltasec`)))))

(fn `TickReady`
  (params (DeltaSec :type "Float (single-precision)"))
  (`|ExecutionSequence`
    (:`then_0`
      (`/Engine/EditorBlueprintResources/ActorMacros.Switch Has Authority`
        (:`Authority`
          (set `self.Deltasec` (* DeltaSec (`self.Deltasec`))))))
    (:`then_1`
      ; 리슨서버- 다 보내야하는 정보:
      ; 서버 자체도 클라여서 ㅇ시퀀ㄱ스연결
      (`self.DS_DeltaSec` (`self.Deltasec`)))))

(fn `UserConstructionScript`)