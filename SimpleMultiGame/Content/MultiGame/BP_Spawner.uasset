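; BP_Spawner is a server-authoritative spawner that creates an item of a configured class at its own transform on BeginPlay.
; If the spawned actor is invalid, SpawnItem sets a five-second SpawnItem timer and binds an OnDestroyed event on that same invalid reference.
; EventDestroy also sets that timer, apparently for respawning.
; Both timers target the spawned or destroyed actor instead of the spawner, so respawning likely fails.
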(event `self.ReceiveBeginPlay`
  (`self.SpawnItem`))

(fn `EventDestroy`
  (params (DestroyedActor :type "Actor Object Reference"))
  (`KismetSystemLibrary.K2_SetTimer` DestroyedActor "SpawnItem" 5.0))

(fn `SpawnItem`
  (`/Engine/EditorBlueprintResources/ActorMacros.Switch Has Authority`
    (:`Authority`
      (bind _returnvalue (`|SpawnActorFromClass` (`|GetArrayItem` (`self.Class`)) (`self.GetTransform`) "Undefined" "MultiplyWithRoot" null null))
      (`/Engine/EditorBlueprintResources/StandardMacros.IsValid` _returnvalue
        (:`Is Not Valid`
          (`KismetSystemLibrary.K2_SetTimer` _returnvalue "SpawnItem" 5.0)
          (add `self.OnDestroyed` _returnvalue (`|CreateDelegate` :!event `EventDestroy`)))))))

(fn `UserConstructionScript`)