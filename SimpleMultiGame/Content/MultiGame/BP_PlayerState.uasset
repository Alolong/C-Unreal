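; BP_PlayerState is a multiplayer PlayerState that tracks a player's collected item count and win or lose result.
; On BeginPlay it registers with BP_GM through BindPS.
; CountItem increments Count until the ten-item cap, after which further calls fire the winner-detection dispatcher.
; UpdateWinner sets IsWin from the count, and RepNotifies on Count and IsWin broadcast changes through dispatchers.
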(event `self.ReceiveBeginPlay`
  ; 내가 생성되면서 나를 등록
  (bind _asbp_gm (cast `/Game/MultiGame/BP_GM` (`GameplayStatics.GetGameMode`)))
  (`/Game/MultiGame/BP_GM.BindPS` _asbp_gm self))

(fn `CountItem`
  (returns (`is count` :type Boolean))
  (if (`self.isFullCount`)
    (`self.DSDetectWinner`)
    (return false)
    (else
      (set `self.Count` (+ (`self.Count`) 1))
      (return true))))

(fn `isFullCount`
  (returns (IsFullCount :type Boolean))
  (return (== (`self.Count`) 10)))

(fn `OnRep_Count`
  ; 게임플레이어스테이트 -RefNotify랑 한몸
  (`self.DSCountItem` (`self.Count`)))

(fn `OnRep_IsWin`
  (`self.DSIsWin` (`self.IsWin`)))

(fn `UpdateWinner`
  (if (>= (`self.Count`) 10)
    (set `self.IsWin` "NewEnumerator1")
    (else
      (set `self.IsWin` "NewEnumerator2"))))

(fn `UserConstructionScript`)