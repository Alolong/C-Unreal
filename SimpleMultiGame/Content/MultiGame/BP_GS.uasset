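; Multiplayer game state Blueprint that tracks the Ready and Start phases and the time elapsed in the current phase.
; ChangeGS sets the RepNotify phase and resets the timer, and the OnRep broadcasts the new phase through a dispatcher.
; Tick routes to a handler per phase; both currently add delta time to the replicated timer on the authority only, then broadcast the total on server and clients.
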(event `self.ReceiveTick`
  (params (DeltaSeconds :type "Float (single-precision)"))
  (switch `/Game/MultiGame/EN_GS` (`self.GameStates`)
    (:`NewEnumerator1`
      (`self.TickReady` DeltaSeconds))
    (:`NewEnumerator2`
      (`self.TickPlay` DeltaSeconds))))

(fn `ChangeGS`
  (params (GameStates :type "/Game/MultiGame/EN_GS Enum" :default "NewEnumerator0"))
  ; refNotify
  (set `self.GameStates` GameStates)
  ; 초기화
  (set `self.TotalDeltaSec` 0.0))

(fn `OnRep_GameStates`
  (`self.DS_ChangeGS` (`self.GameStates`)))

(fn `TickPlay`
  (params (DeltaSec :type "Float (double-precision)"))
  (`|ExecutionSequence`
    (:`then_0`
      ; 서버에서
      (`/Engine/EditorBlueprintResources/ActorMacros.Switch Has Authority`
        (:`Authority`
          ; Replicated
          (set `self.TotalDeltaSec` (+ (`self.TotalDeltaSec`) DeltaSec)))))
    (:`then_1`
      ; 클라+서버
      (`self.DS_TotalDeltaSec` (`self.TotalDeltaSec`)))))

(fn `TickReady`
  (params (DeltaSec :type "Float (double-precision)"))
  (`|ExecutionSequence`
    (:`then_0`
      ; 서버에서
      (`/Engine/EditorBlueprintResources/ActorMacros.Switch Has Authority`
        (:`Authority`
          ; Replicated
          (set `self.TotalDeltaSec` (+ (`self.TotalDeltaSec`) DeltaSec)))))
    (:`then_1`
      ; 클라+서버
      (`self.DS_TotalDeltaSec` (`self.TotalDeltaSec`)))))

(fn `UserConstructionScript`)