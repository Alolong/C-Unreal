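; BP_GM is a multiplayer game mode that drives the match through Ready, Start and End states on BP_GS.
; It binds to the game state's change and elapsed-time dispatchers, sets Ready on BeginPlay, then switches to Start after a short delay.
; BindPS hooks a player state's winner-detection dispatcher.
; UpdateWin calls UpdateWinner on every BP_PlayerState, then sets the state to End.
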(event `self.ReceiveBeginPlay`
  ; Bind GS
  ;; 게임 스테이트(게임상태) 변경
  (bind _asbp_gs (cast `/Game/MultiGame/BP_GS` (`GameplayStatics.GetGameState`)))
  ;; GS에서 생성된 디스패쳐 : Start로 변경
  (add `/Game/MultiGame/BP_GS.DS_ChangeGS` _asbp_gs (`|CreateDelegate` :!event `EV_ChangeGS`))
  (add `/Game/MultiGame/BP_GS.DS_TotalDeltaSec` _asbp_gs (`|CreateDelegate` :!event `EV_TotalDeltaSec`))
  (`/Game/MultiGame/BP_GS.ChangeGS` _asbp_gs "NewEnumerator1")
  (`self.BindPS` null))

(fn `BindPS`
  (params (PS :type "/Game/MultiGame/BP_PlayerState Object Reference"))
  (add `/Game/MultiGame/BP_PlayerState.DSDetectWinner` PS (`|CreateDelegate` :!event `UpdateWin`)))

(fn `EV_ChangeGS`
  (params (GS :type "/Game/MultiGame/EN_GS Enum" :default "NewEnumerator0"))
  ; 변경된 게임 상태 변수로 저장
  (bind _output_get (set `self.GS` GS))
  (`KismetSystemLibrary.PrintString` (`KismetStringLibrary.Concat_StrStr` "Cur Game State Is :" (`|GetEnumeratorNameAsString` _output_get))))

(fn `EV_TotalDeltaSec`
  (params (TotalDeltaSec :type "Float (double-precision)"))
  (switch `/Game/MultiGame/EN_GS` (`self.GS`)
    (:`NewEnumerator1`
      (if (> TotalDeltaSec 6.0)
        (bind _asbp_gs (cast `/Game/MultiGame/BP_GS` (`GameplayStatics.GetGameState`)))
        (`/Game/MultiGame/BP_GS.ChangeGS` _asbp_gs "NewEnumerator2")))))

(fn `UpdateWin`
  (`KismetSystemLibrary.PrintString` "Detectwinner")
  (`|ExecutionSequence`
    (:`then_0`
      (bind _outactors (`GameplayStatics.GetAllActorsOfClass` "/Game/MultiGame/BP_PlayerState.BP_PlayerState_C"))
      ; 뒤에 놓침
      (for _array_element _outactors
        (`/Game/MultiGame/BP_PlayerState.UpdateWinner` _array_element)))
    (:`then_1`
      (bind _asbp_gs (cast `/Game/MultiGame/BP_GS` (`GameplayStatics.GetGameState`)))
      (`/Game/MultiGame/BP_GS.ChangeGS` _asbp_gs "NewEnumerator3"))))

(fn `UserConstructionScript`)